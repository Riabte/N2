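; BP_Barry_purbkle is a purple berry inventory pickup that the player collects by overlap.
; When its Box component begins an overlap, it casts player character 0 to Playr_charatacter and checks whether slot Espaco3 is empty.
; If empty, it destroys the berry actor and writes the item ID into that slot; otherwise the berry stays.
; The overlapping actor itself is never checked.
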(event OnComponentBeginOverlap(Box)
  (params (OverlappedComponent :type Primitive%20Component%20Object%20Reference) (OtherActor :type Actor%20Object%20Reference) (OtherComp :type Primitive%20Component%20Object%20Reference) (OtherBodyIndex :type Integer) (bFromSweep :type Boolean) (SweepResult :type Hit%20Result%20Structure%20%28by%20ref%29))
  ;[1 1 1] quando objeto sopropõe o jogador é coletado e destruido se não houver nada n slot.
  (bind _asplayr_charatacter (Utilities|Casting|CastToPlayr_charatacter (Game|GetPlayerCharacter 0)))
  (if (== (Variables|/Game/Blueprint/character/Playr_charatacter.Playr_charatacter_C|Getespaco3 _asplayr_charatacter) 0)
    (Actor|DestroyActor (Components|GetOwner (Variables|Default|Getbarry_purble)))
    (bind _asplayr_charatacter_2 (Utilities|Casting|CastToPlayr_charatacter (Game|GetPlayerCharacter 0)))
    (if (== (Variables|/Game/Blueprint/character/Playr_charatacter.Playr_charatacter_C|Getespaco3 _asplayr_charatacter_2) 0)
      (Variables|/Game/Blueprint/character/Playr_charatacter.Playr_charatacter_C|Setespaco3 _asplayr_charatacter_2 3))))

(event EventBeginPlay)

(event Collision|EventActorBeginOverlap
  (params (OtherActor :type Actor%20Object%20Reference)))

(event EventTick
  (params (DeltaSeconds :type Float%20%28single-precision%29)))

(fn ConstructionScript)
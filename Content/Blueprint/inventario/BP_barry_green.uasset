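; BP_barry_green is a green berry inventory pickup triggered by its Box overlap.
; On overlap it destroys itself, then writes item ID 2 into the first empty slot among the player character's four Espaco variables.
; It does not check which actor overlapped, always targeting player 0, and the berry is lost when all slots are full.
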(event OnComponentBeginOverlap(Box)
  (params (OverlappedComponent :type Primitive%20Component%20Object%20Reference) (OtherActor :type Actor%20Object%20Reference) (OtherComp :type Primitive%20Component%20Object%20Reference) (OtherBodyIndex :type Integer) (bFromSweep :type Boolean) (SweepResult :type Hit%20Result%20Structure%20%28by%20ref%29))
  (Actor|DestroyActor (Components|GetOwner (Variables|Default|Getass_barry_green)))
  (bind _asplayr_charatacter (Utilities|Casting|CastToPlayr_charatacter (Game|GetPlayerCharacter 0)))
  (if (== (Variables|/Game/Blueprint/character/Playr_charatacter.Playr_charatacter_C|Getespaco1 _asplayr_charatacter) 0)
    (Variables|/Game/Blueprint/character/Playr_charatacter.Playr_charatacter_C|Setespaco1 _asplayr_charatacter 2)
    (elif (== (Variables|/Game/Blueprint/character/Playr_charatacter.Playr_charatacter_C|Getespaco2 _asplayr_charatacter) 0)
      (Variables|/Game/Blueprint/character/Playr_charatacter.Playr_charatacter_C|Setespaco2 _asplayr_charatacter 2)
      (elif (== (Variables|/Game/Blueprint/character/Playr_charatacter.Playr_charatacter_C|Getespaco3 _asplayr_charatacter) 0)
        (Variables|/Game/Blueprint/character/Playr_charatacter.Playr_charatacter_C|Setespaco3 _asplayr_charatacter 2)
        (elif (== (Variables|/Game/Blueprint/character/Playr_charatacter.Playr_charatacter_C|Getespaco4 _asplayr_charatacter) 0)
          (Variables|/Game/Blueprint/character/Playr_charatacter.Playr_charatacter_C|Setespaco4 _asplayr_charatacter 2))))))

(event EventBeginPlay)

(event Collision|EventActorBeginOverlap
  (params (OtherActor :type Actor%20Object%20Reference)))

(event EventTick
  (params (DeltaSeconds :type Float%20%28single-precision%29)))

(fn ConstructionScript)
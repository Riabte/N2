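; Light source actor built to drive a day/night style sun rotation alongside the level's BP_Sky and SkyLight.
; BeginPlay caches the first BP_Sky and SkyLight found in the world.
; A timeline's update would set the actor's pitch, refresh the sky's sun direction and set skylight intensity from its curves, but nothing starts the timeline, so that logic never runs.
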(event EventBeginPlay
  (bind _outactors (Actor|GetAllActorsOfClass "/Game/Blueprint/BP_Sky.BP_Sky_C"))
  (Variables|Default|SetS_Ref (Utilities|Array|Get(acopy) _outactors))
  (bind _outactors_2 (Actor|GetAllActorsOfClass "/Script/Engine.SkyLight"))
  (Variables|Default|SetS_L_ref (Utilities|Array|Get(acopy) _outactors_2)))

(fn ConstructionScript)